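; BP_Debris is a catchable piece of debris, owned by a BP_DebrisField, that yields a Value when caught.
; Construction sizes its collision sphere and scales a second sphere component from Radius.
; BeginPlay caches a squared kill distance just beyond the field's radius, and Tick destroys the actor once its squared distance from the world origin exceeds it.
; Catch destroys the debris and returns its Value.
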(event `self.ReceiveBeginPlay`
  (bind _asbp_debris_field (cast `/Game/Blueprints/BP_DebrisField` (`self.GetOwner`)))
  (bind _returnvalue (+ (`/Game/Blueprints/BP_DebrisField.Radius` _asbp_debris_field) 1.0))
  (set `self.KillDistance` (* _returnvalue _returnvalue)))

(event `self.ReceiveTick`
  (params (DeltaSeconds :type "Float (single-precision)"))
  (if (> (`KismetMathLibrary.VSizeSquared` (`self.K2_GetActorLocation`)) (`self.KillDistance`))
    (`self.K2_DestroyActor`)))

(fn `Catch`
  (returns (Value :type "Float (double-precision)"))
  (`self.K2_DestroyActor`)
  (return (`self.Value`)))

(fn `UserConstructionScript`
  (`SphereComponent.SetSphereRadius` (`self.Sphere`) (`self.Radius`) false)
  (`SceneComponent.SetRelativeScale3D` (`self.Sphere1`) (`KismetMathLibrary.Conv_DoubleToVector` (/ (`self.Radius`) 50.0))))