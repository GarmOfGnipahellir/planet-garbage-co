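; BP_DebrisField is a spawner that creates random debris actors around a sphere, at a rate that changes with game time.
; Each Tick rolls against a spawn chance lerped from min to max over fifteen minutes and divided by the tick interval.
; Debris spawns on a horizontal ring at Radius, aimed within a cone toward the center plus a fixed rotation offset.
; The construction script matches the sphere's radius to Radius.
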(event `self.ReceiveTick`
  (params (DeltaSeconds :type "Float (single-precision)"))
  (bind _debris (`self.Debris`))
  (bind _returnvalue (+ (`SceneComponent.K2_GetComponentLocation` (`self.Sphere`)) (* (`KismetMathLibrary.Vector_Normal2D` (`KismetMathLibrary.RandomUnitVector`)) (`self.Radius`))))
  (set `self.SpawnChance` (`KismetMathLibrary.Lerp` (`self.SpawnChanceMin`) (`self.SpawnChanceMax`) (/ (`KismetSystemLibrary.GetGameTimeInSeconds`) (* 60.0 15.0))))
  (if (< (`KismetMathLibrary.RandomFloat`) (/ (`self.SpawnChance`) (`self.GetActorTickInterval`)))
    (`|SpawnActorFromClass` (`|GetArrayItem` _debris (`KismetMathLibrary.RandomIntegerInRange` 0 (- (`KismetArrayLibrary.Array_Length` _debris) 1))) (`KismetMathLibrary.MakeTransform` _returnvalue (`KismetMathLibrary.ComposeRotators` (`KismetMathLibrary.Conv_VectorToRotator` (`KismetMathLibrary.RandomUnitVectorInConeInDegrees` (`KismetMathLibrary.GetDirectionUnitVector` _returnvalue (`SceneComponent.K2_GetComponentLocation` (`self.Sphere`))) 45.0)) (struct :`Yaw` 15.0))) "Undefined" "OverrideRootScale" self null)))

(fn `UserConstructionScript`
  (`SphereComponent.SetSphereRadius` (`self.Sphere`) (`self.Radius`) true))