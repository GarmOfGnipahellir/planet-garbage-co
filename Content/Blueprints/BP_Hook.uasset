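; Thrown hook actor that catches BP_Debris and reels it back, drawing a Niagara beam to world origin.
; The Throw timeline moves it from spawn toward its forward vector times Range, then reverses.
; Overlapping debris stops both, and a Catch timeline snaps the hook onto it, plays a hit sound, then reverses Throw to drag it back.
; On return it calls CallReturn, destroys itself and puts any catch at world origin.
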(event `self.ReceiveBeginPlay`
  (bind _niagara (`self.Niagara`))
  (bind _catched (`self.Catched`))
  (bind _catched_2 (`self.Catched`))
  (set `self.Origin` (`self.K2_GetActorLocation`))
  (set `self.Target` (* (`self.GetActorForwardVector`) (`self.Range`)))
  (`TimelineComponent.SetPlayRate` (`self.Throw`) (/ (`self.Speed`) (`self.Range`)))
  (bind (_direction _alpha) (`Timeline|Throw` :!via `PlayFromStart`)
    (:`Update`
      (`|ExecutionSequence`
        (:`then_0`
          (`NiagaraComponent.SetNiagaraVariableVec3` _niagara "User.Beam Start" (`SceneComponent.K2_GetComponentLocation` (`self.Scene`)) :!label _label)
          (`NiagaraComponent.SetNiagaraVariableVec3` _niagara "User.Beam End" (0.0 0.0 0.0)))
        (:`then_1`
          (bind _returnvalue (`KismetMathLibrary.VLerp` (`self.Origin`) (`self.Target`) _alpha))
          (`self.K2_SetActorLocation` _returnvalue)
          (if (and (== _direction 1) (`TimelineComponent.IsPlaying` (`self.Throw`)))
            (`/Engine/EditorBlueprintResources/StandardMacros.IsValid` _catched
              (:`Is Valid`
                (`self.K2_SetActorLocation` _catched _returnvalue false false)))))))
    (:`Finished`
      (if (== _direction 0)
        (`TimelineComponent.Reverse` (`self.Throw`))
        (else
          (`self.Return`)
          (`self.K2_DestroyActor`)
          (if (`self.HasCatched`)
            (`/Engine/EditorBlueprintResources/StandardMacros.IsValid` _catched_2
              (:`Is Valid`
                (`self.K2_SetActorLocation` _catched_2 (0.0 0.0 0.0) false false)))))))))

(event `self.Sphere1.OnComponentBeginOverlap`
  (params (OverlappedComponent :type "PrimitiveComponent Object Reference") (OtherActor :type "Actor Object Reference") (OtherComp :type "PrimitiveComponent Object Reference") (OtherBodyIndex :type Integer) (bFromSweep :type Boolean) (SweepResult :type "HitResult Structure (by ref)"))
  (bind _target (`self.Target`))
  (`/Engine/EditorBlueprintResources/StandardMacros.IsValid` (`self.Catched`)
    (:`Is Not Valid`
      (bind _asbp_debris (cast `/Game/Blueprints/BP_Debris` OtherActor))
      (set `self.Catched` _asbp_debris)
      (set `/Game/Blueprints/BP_Debris.IsCatched` true _asbp_debris)
      (set `self.HasCatched` true)
      (`MovementComponent.StopMovementImmediately` (`/Game/Blueprints/BP_Debris.ProjectileMovement` _asbp_debris))
      (set `self.Target` (`self.K2_GetActorLocation` _asbp_debris))
      (set `self.CatchLocation` (`self.K2_GetActorLocation`))
      (`TimelineComponent.Stop` (`self.Throw`))
      (bind (_direction _alpha) (`Timeline|Catch`)
        (:`Update`
          (`self.K2_SetActorLocation` (`KismetMathLibrary.VLerp` (`self.CatchLocation`) _target _alpha))
          (`self.K2_SetActorRotation` (`KismetMathLibrary.FindLookAtRotation` (`self.Origin`) (`self.Target`)))
          (goto _label))
        (:`Finished`
          (`GameplayStatics.PlaySoundAtLocation` "/Game/Audio/Hit_01_Cue.Hit_01_Cue" _target (struct) 1.0 1.0 0.0 null null null)
          (`KismetSystemLibrary.Delay` 0.1)
          (`TimelineComponent.Reverse` (`self.Throw`)))))))

(fn `UserConstructionScript`)