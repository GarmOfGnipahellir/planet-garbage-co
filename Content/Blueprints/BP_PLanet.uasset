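; BP_PLanet is the player's planet, which launches hooks toward the mouse cursor and banks debris that touches it into PlayerState.
; ShootHook spawns BP_Hook at the planet's edge, aimed via a ray-to-ground-plane cursor intersection, with range and speed scaled by upgrades.
; Hooks are limited to one until return unless MultiHook is owned; SpiderHook adds an evenly spaced radial burst.
; The construction script sizes collision and mesh from Radius.
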(event `self.ReceiveBeginPlay`
  (bind _asbp_player_state (cast `/Game/Blueprints/BP_PlayerState` (`Controller.PlayerState` (`GameplayStatics.GetPlayerController` 0))))
  (set `self.PlayerState` _asbp_player_state))

(event `self.Sphere.OnComponentBeginOverlap`
  (params (OverlappedComponent :type "PrimitiveComponent Object Reference") (OtherActor :type "Actor Object Reference") (OtherComp :type "PrimitiveComponent Object Reference") (OtherBodyIndex :type Integer) (bFromSweep :type Boolean) (SweepResult :type "HitResult Structure (by ref)"))
  (bind _asbp_debris (cast `/Game/Blueprints/BP_Debris` OtherActor))
  (bind _value (`/Game/Blueprints/BP_Debris.Catch` _asbp_debris))
  (`/Game/Blueprints/BP_PlayerState.Add Value` (`self.PlayerState`) _value)
  (`GameplayStatics.PlaySoundAtLocation` "/Game/Audio/Pickup_01_Cue.Pickup_01_Cue" (0.0 0.0 0.0) (struct) 1.0 1.0 0.0 null null null))

(event `ShootHook`
  (bind _numspiderhook (`self.NumSpiderHook`))
  (bind _returnvalue (`KismetMathLibrary.GetDirectionUnitVector` (`self.K2_GetActorLocation`) (`self.Get Cursor World Location`)))
  (if (or (not (`self.IsHookActive`)) (`/Game/Blueprints/BP_PlayerState.HasMultiHook` (`self.PlayerState`)))
    (`|ExecutionSequence`
      (:`then_0`
        (if (`/Game/Blueprints/BP_PlayerState.HasSpiderHook` (`self.PlayerState`))
          (for _index (range _numspiderhook)
            (bind _returnvalue_2 (`KismetMathLibrary.MakeRotator` 0.0 0.0 (* _index (/ 360.0 (`KismetMathLibrary.Conv_IntToDouble` _numspiderhook)))))
            (`|SpawnActorFromClass` "/Game/Blueprints/BP_Hook.BP_Hook_C" (`KismetMathLibrary.MakeTransform` (+ (`self.K2_GetActorLocation`) (* (`KismetMathLibrary.GetForwardVector` _returnvalue_2) (`self.Radius`))) _returnvalue_2) "Undefined" "OverrideRootScale" null (+ (* (`/Game/Blueprints/BP_PlayerState.HookRangeUpgrades` (`self.PlayerState`)) 50.0) 200.0) (+ (* (`/Game/Blueprints/BP_PlayerState.HookSpeedUpgrades` (`self.PlayerState`)) 50.0) 400.0) null))))
      (:`then_1`
        (bind _returnvalue_3 (`|SpawnActorFromClass` "/Game/Blueprints/BP_Hook.BP_Hook_C" (`KismetMathLibrary.MakeTransform` (+ (`self.K2_GetActorLocation`) (* _returnvalue (`self.Radius`))) (`KismetMathLibrary.Conv_VectorToRotator` _returnvalue)) "Undefined" "OverrideRootScale" null (+ (* (`/Game/Blueprints/BP_PlayerState.HookRangeUpgrades` (`self.PlayerState`)) 50.0) 200.0) (+ (* (`/Game/Blueprints/BP_PlayerState.HookSpeedUpgrades` (`self.PlayerState`)) 50.0) 400.0) null))
        (set `self.IsHookActive` true)
        (add `/Game/Blueprints/BP_Hook.Return` _returnvalue_3 (delegate `OnHookReturned`))
        (`GameplayStatics.PlaySoundAtLocation` "/Game/Audio/Launch_01_Cue.Launch_01_Cue" (0.0 0.0 0.0) (struct) 1.0 1.0 0.0 null null null)))))

(event `OnHookReturned`
  (set `self.IsHookActive` false))

(event `self.ReceiveTick`
  (params (DeltaSeconds :type "Float (single-precision)"))
  (`SceneComponent.K2_AddLocalRotation` (`self.Sphere1`) (`KismetMathLibrary.MakeRotator` 0.0 0.0 (* DeltaSeconds 30.0)) false false))

(fn `Get Cursor World Location`
  (returns (Intersection :type "Vector Structure"))
  (bind (_worldlocation _worlddirection) (`PlayerController.DeprojectMousePositionToWorld` (`GameplayStatics.GetPlayerController` 0)))
  (return (`.Intersection` (`KismetMathLibrary.LinePlaneIntersection` _worldlocation (+ _worldlocation (* _worlddirection 10000.0)) (`KismetMathLibrary.MakePlaneFromPointAndNormal` (0.0 0.0 0.0) (0.0 0.0 1.0))))))

(fn `UserConstructionScript`
  (`SphereComponent.SetSphereRadius` (`self.Sphere`) (+ (`self.Radius`) 10.0) false)
  (`SceneComponent.SetRelativeScale3D` (`self.Sphere1`) (`KismetMathLibrary.Conv_DoubleToVector` (/ (`self.Radius`) 50.0))))