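; Player pawn that acts as an input relay to the BP_Planet actor, firing its hook on left click.
; BeginPlay takes the first BP_Planet found and enables player input on it, and left mouse calls ShootHook on that planet.
; Right mouse only sets a held flag, as the drag-movement logic that reads it is disconnected.
; Cursor-trace planet picking, PlanetMenu creation and Sentry plane reveal are also unwired leftovers.
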(event `self.ReceiveBeginPlay`
  (bind _outactors (`GameplayStatics.GetAllActorsOfClass` "/Game/Blueprints/BP_PLanet.BP_Planet_C"))
  (bind _output_get (set `self.Planet` (`|GetArrayItem` _outactors)))
  (`self.EnableInput` _output_get (`GameplayStatics.GetPlayerController` 0)))

(event `InputAxisKey|MouseX`
  (params (AxisValue :type "Float (single-precision)")))

(event `InputAxisKey|MouseY`
  (params (AxisValue :type "Float (single-precision)")))

(event `Key|RightMouseButton`
  (params (Key :type "Key Structure"))
  (:`Pressed`
    (set `self.IsRMBDown` true))
  (:`Released`
    (set `self.IsRMBDown` false)))

(event `self.ReceiveTick`
  (params (DeltaSeconds :type "Float (single-precision)")))

(event `Key|LeftMouseButton`
  (params (Key :type "Key Structure"))
  (:`Pressed`
    (`/Game/Blueprints/BP_PLanet.ShootHook` (`self.Planet`))))

(fn `UserConstructionScript`)