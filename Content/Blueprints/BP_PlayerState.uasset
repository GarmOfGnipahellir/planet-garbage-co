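; Player state that holds the player's Worth currency and their grappling hook upgrade progress.
; Upgrade events check a cost function against Worth, deduct it, then raise the range or speed level or unlock the multi-hook or spider hook.
; Range and speed costs grow linearly per level, while each special hook costs double once the other is owned.
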(event `UpgradeHookRange`
  (if (<= (`self.HookRangeCost`) (`self.Worth`))
    (set `self.Worth` (- (`self.Worth`) (`self.HookRangeCost`)))
    (`/Engine/EditorBlueprintResources/StandardMacros.IncrementInt` (`self.HookRangeUpgrades`))))

(event `UpgradeHookSpeed`
  (if (<= (`self.HookSpeedCost`) (`self.Worth`))
    (set `self.Worth` (- (`self.Worth`) (`self.HookSpeedCost`)))
    (`/Engine/EditorBlueprintResources/StandardMacros.IncrementInt` (`self.HookSpeedUpgrades`))))

(event `UpgradeMultiHook`
  (if (<= (`self.HookMultiCost`) (`self.Worth`))
    (set `self.Worth` (- (`self.Worth`) (`self.HookMultiCost`)))
    (set `self.HasMultiHook` true)))

(event `UpgradeSpiderHook`
  (if (<= (`self.HookSpiderCost`) (`self.Worth`))
    (set `self.Worth` (- (`self.Worth`) (`self.HookSpiderCost`)))
    (set `self.HasSpiderHook` true)))

(fn `Add Value`
  (params (Value :type "Float (double-precision)"))
  (set `self.Worth` (+ Value (`self.Worth`))))

(fn `HookMultiCost`
  (returns (`Return Value` :type "Float (double-precision)"))
  (return (select `bool` (`self.HasSpiderHook`) :`false` 2000.0 :`true` 4000.0 :!type "Float (single-precision)")))

(fn `HookRangeCost`
  (returns (`Return Value` :type "Float (double-precision)"))
  (return (+ (* (`self.HookRangeUpgrades`) (`self.HookRangeCostPL`)) 50.0)))

(fn `HookSpeedCost`
  (returns (`Return Value` :type "Float (double-precision)"))
  (return (+ (* (`self.HookSpeedUpgrades`) (`self.HookSpeedCostPL`)) 20.0)))

(fn `HookSpiderCost`
  (returns (`Return Value` :type "Float (double-precision)"))
  (return (select `bool` (`self.HasMultiHook`) :`false` 3000.0 :`true` 6000.0 :!type "Float (single-precision)")))

(fn `UserConstructionScript`)